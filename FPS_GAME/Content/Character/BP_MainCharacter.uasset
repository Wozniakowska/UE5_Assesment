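; BP_MainCharacter is the player character, handling the game-over check and timer pickups.
; Every Tick it compares PlayerHealth to NumCheck, and at or below it pauses the game, shows the WB_GameOver widget and switches to UI-only input with a cursor.
; Capsule overlaps with actors tagged "Timer" add time to Seconds.
; A similar "Health" tag branch that would raise PlayerHealth is disconnected and never runs.
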(event OnComponentBeginOverlap(CapsuleComponent)
  (params (OverlappedComponent :type Primitive%20Component%20Object%20Reference) (OtherActor :type Actor%20Object%20Reference) (OtherComp :type Primitive%20Component%20Object%20Reference) (OtherBodyIndex :type Integer) (bFromSweep :type Boolean) (SweepResult :type Hit%20Result%20Structure%20%28by%20ref%29))
  (if (Actor|ActorHasTag OtherActor "Timer")
    (Variables|Default|SetSeconds (+ (Variables|Default|GetSeconds) 1e+01))))

(event EventBeginPlay)

(event Collision|EventActorBeginOverlap
  (params (OtherActor :type Actor%20Object%20Reference)))

(event EventTick
  (params (DeltaSeconds :type Float%20%28single-precision%29))
  (bind _returnvalue (Game|GetPlayerController 0))
  (if (<= (Variables|Default|GetPlayerHealth) (Variables|Default|GetNumCheck))
    (Game|SetGamePaused true)
    (bind _returnvalue_2 (UserInterface|CreateWidget "/Game/Widgets_UI/WB_GameOver.WB_GameOver_C"))
    (UserInterface|Viewport|AddtoViewport _returnvalue_2 0)
    (Input|SetInputModeUIOnly _returnvalue 0 "DoNotLock" false)
    (Variables|/Script/Engine.PlayerController|SetbShowMouseCursor _returnvalue true)))

(fn ConstructionScript)